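; BP_Destructable is an obstacle that BP_Shot projectiles can destroy after a number of hits.
; A Box overlap destroys the incoming shot and briefly flashes the PaperSprite to DestroyColor before restoring OriginalColor.
; After the flash delay it increments HitCounter, destroying the actor with SE_Attack once Toughness is reached and otherwise playing SE_Break.
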(event OnComponentBeginOverlap(Box)
  (params (OverlappedComponent :type Primitive%20Component%20Object%20Reference) (OtherActor :type Actor%20Object%20Reference) (OtherComp :type Primitive%20Component%20Object%20Reference) (OtherBodyIndex :type Integer) (bFromSweep :type Boolean) (SweepResult :type Hit%20Result%20Structure%20%28by%20ref%29))
  (bind _asbp_shot (Utilities|Casting|CastToBP_Shot OtherActor))
  (Actor|DestroyActor _asbp_shot)
  (Sprite|SetSpriteColor (Variables|Default|GetPaperSprite) (Variables|Default|GetDestroyColor))
  (Utilities|FlowControl|Delay 0.05)
  (Sprite|SetSpriteColor (Variables|Default|GetPaperSprite) (Variables|Default|GetOriginalColor))
  (Variables|Default|SetHitCounter (+ (Variables|Default|GetHitCounter) 1))
  (if (>= (Variables|Default|GetHitCounter) (Variables|Default|GetToughness))
    (Audio|PlaySound2D "/Game/TutorialProject/Sounds/SoundEffects/SE_Attack.SE_Attack")
    (Actor|DestroyActor)
    (else
      (Audio|PlaySound2D "/Game/TutorialProject/Sounds/SoundEffects/SE_Break.SE_Break"))))

(event EventBeginPlay)

(event Collision|EventActorBeginOverlap
  (params (OtherActor :type Actor%20Object%20Reference)))

(event EventTick
  (params (DeltaSeconds :type Float%20%28single-precision%29)))

(fn ConstructionScript)