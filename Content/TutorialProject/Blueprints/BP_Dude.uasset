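; BP_Dude is the player character of a 2D side-scrolling platformer, handling movement, upgrade-gated double jump and shooting, ladder climbing, springs and damage.
; Input and events set a State enum that UpdateAnimation, also run on Tick, maps to sprite flipbooks.
; Weapon cycling reads data table rows, whose color and scale are applied to spawned BP_Shot projectiles.
; Enemy overlap applies knockback, health loss and a dynamic-material hit flash.
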(event OnComponentBeginOverlap(Box)
  (params (OverlappedComponent :type Primitive%20Component%20Object%20Reference) (OtherActor :type Actor%20Object%20Reference) (OtherComp :type Primitive%20Component%20Object%20Reference) (OtherBodyIndex :type Integer) (bFromSweep :type Boolean) (SweepResult :type Hit%20Result%20Structure%20%28by%20ref%29))
  (Utilities|Casting|CastToBP_Enemy_Patroller OtherActor)
  (CallFunction|DamageSystem (Variables|Default|GetStandardDamage)))

(event Custom|ClimbingEnd
  ;[0 1 0.2318] Handle Climbing
  (Variables|Default|SetState "NewEnumerator0")
  (CallFunction|UpdateAnimation)
  (Pawn|Components|CharacterMovement|SetMovementMode (Variables|Character|GetCharacterMovement) "MOVE_Walking" 0))

(event Custom|UpdateAnimation
  (bind _sprite (Variables|Default|GetSprite))
  ;[0 1 0.2318] Animation State Machine
  (switch Utilities|FlowControl|Switch|SwitchonCharacterStates (Variables|Default|GetState)
    (:NewEnumerator0
      (if (not (Variables|Default|GetIsDead))
        (Sprite|SetFlipbook (Variables|Default|GetSprite) (select (> (Math|Vector|VectorLength (Transformation|GetVelocity)) 0.0) "/Game/TutorialProject/Sprites/Characters/Megaman_Assets/AM_Running.AM_Running" "/Game/TutorialProject/Sprites/Characters/Megaman_Assets/AM_Standing.AM_Standing"))))
    (:NewEnumerator2
      (Sprite|SetFlipbook (Variables|Default|GetSprite) "/Game/TutorialProject/Sprites/Characters/Megaman_Assets/AM_Jumping.AM_Jumping"))
    (:NewEnumerator4
      (Transformation|AddActorLocalRotation "0,180.000000, 0" false false)
      (Sprite|SetFlipbook (Variables|Default|GetSprite) "/Game/TutorialProject/Sprites/Characters/Megaman_Assets/AM_Hurt.AM_Hurt"))
    (:NewEnumerator5
      (Sprite|SetFlipbook (Variables|Default|GetSprite) "/Game/TutorialProject/Sprites/Characters/A_Dead.A_Dead"))
    (:NewEnumerator6
      (if (Variables|Default|GetIsDead)
        (Sprite|SetFlipbook (Variables|Default|GetSprite) "/Game/TutorialProject/Sprites/Characters/A_Dead.A_Dead")
        (else
          (Transformation|AddActorLocalRotation "0,180.000000, 0" false false)
          (Sprite|SetFlipbook (Variables|Default|GetSprite) "/Game/TutorialProject/Sprites/Characters/A_Sitting.A_Sitting"))))
    (:NewEnumerator7
      (Sprite|SetFlipbook (Variables|Default|GetSprite) "/Game/TutorialProject/Sprites/Characters/Megaman_Assets/AM_StandShot.AM_StandShot"))
    (:NewEnumerator1
      (Sprite|SetFlipbook (Variables|Default|GetSprite) "/Game/TutorialProject/Sprites/Characters/Megaman_Assets/AM_RunShot.AM_RunShot"))
    (:NewEnumerator9
      (Sprite|SetFlipbook (Variables|Default|GetSprite) "/Game/TutorialProject/Sprites/Characters/Megaman_Assets/AM_JumpShot.AM_JumpShot"))
    (:NewEnumerator8
      (Sprite|SetFlipbook (Variables|Default|GetSprite) "/Game/TutorialProject/Sprites/Characters/Megaman_Assets/AM_Climbing.AM_Climbing")
      (if (Math|Float|InRange(Float) (Math|Vector|VectorLength (Transformation|GetVelocity)) -0.1 0.1)
        (Components|Timeline|SetPlayRate _sprite 0.0)
        (else
          (Components|Timeline|SetPlayRate _sprite 1.0))))
    (:NewEnumerator10
      (Sprite|SetFlipbook (Variables|Default|GetSprite) "/Game/TutorialProject/Sprites/Characters/Megaman_Assets/AM_Climbing.AM_Climbing"))))

(event Custom|Ceiling%20Spring
  ;[1 1 1] LaunchPad
  (Variables|Default|SetIsJumping true)
  (Components|Movement|StopMovementImmediately (Variables|Character|GetCharacterMovement))
  (Variables|Default|SetState "NewEnumerator2")
  (Physics|AddForce (Variables|Character|GetCharacterMovement) (Math|Vector|MakeVector 0.0 0.0 "- 5000000"))
  (CallFunction|UpdateAnimation))

(event Custom|Damage%20System
  (params (DamageIn :type Float%20%28single-precision%29))
  ;[0 1 0.2318] Damage System
  (Variables|Default|SetisHit true)
  (Input|DisableInput (Game|GetPlayerController 0))
  (Components|Movement|StopMovementImmediately (Variables|Character|GetCharacterMovement))
  (Variables|Default|SetState "NewEnumerator4")
  (Physics|AddForce (Variables|Character|GetCharacterMovement) (Math|Vector|MakeVector (* (Variables|Default|GetFacing) (Variables|Default|GetKnockback)) 0.0 2.2e+06))
  (Rendering|Material|SetScalarParameterValue (Variables|Default|GetSpriteMaterial) "isHit" 1.0 :!class /Script/Engine.MaterialInstanceDynamic)
  (CallFunction|UpdateAnimation)
  (bind _output_get (Variables|Default|SetHealthCurrent (- (Variables|Default|GetHealthCurrent) DamageIn)))
  (if (<= _output_get 0.0)
    (Variables|Default|SetState "NewEnumerator5")
    (Variables|Default|SetIsDead true))
  (Utilities|FlowControl|Delay 0.5)
  (Rendering|Material|SetScalarParameterValue (Variables|Default|GetSpriteMaterial) "isHit" 0.0 :!class /Script/Engine.MaterialInstanceDynamic)
  (CallFunction|UpdateAnimation))

(event Custom|Spring
  ;[1 1 1] LaunchPad
  (Variables|Default|SetIsJumping true)
  (Components|Movement|StopMovementImmediately (Variables|Character|GetCharacterMovement))
  (Variables|Default|SetState "NewEnumerator2")
  (Physics|AddForce (Variables|Character|GetCharacterMovement) (Math|Vector|MakeVector 0.0 0.0 5e+06))
  (CallFunction|UpdateAnimation))

(event Custom|DetectLadder
  (bind _returnvalue (Transformation|GetActorLocation))
  (bind (_x _y _z) (Math|Vector|BreakVector _returnvalue))
  ;[0 1 0.2318] Handle Climbing
  (bind _outhit (Collision|LineTraceByChannel _returnvalue (Math|Vector|MakeVector _x _y (+ _z (* (Input|AxisValues|GetMoveUp) 2e+01))) "TraceTypeQuery1" false 0 "ForOneFrame"))
  (bind _asbp_ladder (Utilities|Casting|CastToBP_Ladder (.hitactor _outhit)))
  (Default|AllowDown _asbp_ladder)
  (Collision|SetCollisionEnabled (Variables|/Game/TutorialProject/Blueprints/BP_Ladder.BP_Ladder_C|GetStaticMesh _asbp_ladder) "NoCollision"))

(event Custom|InitWeapon
  (bind _outrownames (DataTable|GetDataTableRowNames "/Game/TutorialProject/Blueprints/WeaponData.WeaponData"))
  (bind _output_get (Variables|Default|SetWeaponArray _outrownames))
  (Variables|Default|SetNumberOfWeapons (Utilities|Array|Length _output_get)))

(event EventTick
  (params (DeltaSeconds :type Float%20%28single-precision%29))
  ;[0 0.09126 1] Animator
  (if (Variables|Default|GetIsDead)
    (Variables|Default|SetState "NewEnumerator5")
    (Input|DisableInput (Game|GetPlayerController 0))
    (else
      (CallFunction|UpdateAnimation)
      (Math|Float|CompareFloat (.X (Math|Vector|BreakVector (Variables|/Script/Engine.MovementComponent|GetVelocity (Pawn|GetMovementComponent)))) 0.0
        (:>
          (Pawn|SetControlRotation (Pawn|GetController) (Math|Rotator|MakeRotator 0.0 0.0 0.0)))
        (:<
          (Pawn|SetControlRotation (Pawn|GetController) (Math|Rotator|MakeRotator 0.0 0.0 1.8e+02))))
      (if (not (Variables|Default|GetisHit))
        (if (AI|Components|NavMovement|IsFalling (Variables|Character|GetCharacterMovement))
          (Variables|Default|SetState "NewEnumerator2")
          (Variables|Default|SetIsJumping true))))))

(event EventBeginPlay
  ;[1 0.8283 0] GameSetup
  (Utilities|FlowControl|Sequence
    (:then_0
      (Class|ActorComponent|SetIsReplicated (Variables|Default|GetSprite) true))
    (:then_1
      (bind _returnvalue (UserInterface|CreateWidget "/Game/TutorialProject/Blueprints/Widget_HUD.Widget_HUD_C" (Game|GetPlayerController 0)))
      (bind _output_get (Variables|Default|SetHealthBar _returnvalue))
      (UserInterface|Viewport|AddtoViewport _output_get 0))
    (:then_2
      (CallFunction|InitWeapon))))

(event EventOnLanded
  (params (Hit :type Hit%20Result%20Structure%20%28by%20ref%29))
  ;[0 1 0.2318] Handle Jumping
  (if (Variables|Default|GetisHit)
    (Input|DisableInput (Game|GetPlayerController 0))
    (Utilities|FlowControl|Delay 0.075)
    (Variables|Default|SetisHit false)
    (Variables|Default|SetState "NewEnumerator0")
    (CallFunction|UpdateAnimation)
    (Input|EnableInput (Game|GetPlayerController 0))
    (else
      (Variables|Default|SetState "NewEnumerator0")
      (CallFunction|UpdateAnimation)
      (Utilities|FlowControl|Delay 0.075)))
  (Variables|Default|SetIsJumping false)
  (CallFunction|UpdateAnimation)
  (Utilities|FlowControl|DoN 2) ; enters at Reset
)

(event Input|ActionEvents|InputActionJump
  (params (Key :type Key%20Structure :default "AnyKey"))
  ;[0 1 0.2318] Handle Jumping
  (:Pressed
    (if (.DoubleJump (Utilities|Struct|BreakUpgrades (Variables|Default|GetUpgrades)))
      (bind _counter (Utilities|FlowControl|DoN 2)
        (:Exit
          (switch int _counter
            (:1
              (Audio|SpawnSound2D "/Game/TutorialProject/Sounds/SoundEffects/SE_Shot.SE_Shot" :!label _label)
              (Variables|Default|SetState "NewEnumerator2")
              (Variables|Default|SetIsJumping true)
              (CallFunction|UpdateAnimation)
              (Character|Jump))
            (:2
              (Components|Movement|StopMovementImmediately (Variables|Character|GetCharacterMovement))
              (Character|LaunchCharacter "0, 0,400.000000" false false)
              (Audio|SpawnSound2D "/Game/TutorialProject/Sounds/SoundEffects/SE_Shot.SE_Shot")))))
      (elif (not (Variables|Default|GetIsJumping))
        (goto _label)))))

(event Input|ActionEvents|InputActionShoot
  (params (Key :type Key%20Structure :default "AnyKey"))
  (bind _upgrades (Variables|Default|GetUpgrades))
  (bind _shoot (Utilities|Struct|BreakUpgrades _upgrades))
  ;[1 0.03995 0.0495] Handle Shoot
  (:Pressed
    ;[1 0 0.9957] Debug Mouse Input
    (Rendering|Debug|DrawDebugLine (Transformation|GetWorldLocation (Variables|Default|GetArrow)) (.WorldLocation (Game|Player|ConvertMouseLocationToWorldSpace (Game|GetPlayerController self))) "(R=0.000000,G=0.000000,B=0.000000,A=1.000000)" 0.25 0.0)
    (if _shoot
      (Variables|Default|SetIsShooting true)
      (Audio|PlaySound2D "/Game/TutorialProject/Sounds/SoundEffects/SE_Jump.SE_Jump")
      (if (Variables|Default|GetIsJumping)
        (bind _returnvalue (Game|SpawnActorfromClass "/Game/TutorialProject/Blueprints/Projectiles/BP_Shot.BP_Shot_C" (Transformation|GetWorldTransform (Variables|Default|GetArrow2)) "AlwaysSpawn" 0 0))
        (CallFunction|SetWeaponParameters _returnvalue)
        (Variables|Default|SetState "NewEnumerator9")
        (CallFunction|UpdateAnimation :!label _label)
        (else
          (bind _returnvalue_2 (Game|SpawnActorfromClass "/Game/TutorialProject/Blueprints/Projectiles/BP_Shot.BP_Shot_C" (Transformation|GetWorldTransform (Variables|Default|GetArrow)) "AlwaysSpawn" 0 0))
          (CallFunction|SetWeaponParameters _returnvalue_2)
          (if (> (Math|Vector|VectorLength (Transformation|GetVelocity)) 0.0)
            (Variables|Default|SetisMoving true)
            (if (and (Variables|Default|GetisMoving) (Variables|Default|GetIsShooting))
              (Variables|Default|SetState "NewEnumerator1")
              (goto _label))
            (else
              (Variables|Default|SetisMoving false)
              (Variables|Default|SetState "NewEnumerator7")
              (goto _label)))))))
  (:Released
    (if _shoot
      (Utilities|FlowControl|RetriggerableDelay 0.25)
      (Variables|Default|SetIsShooting false)
      (if (AI|Components|NavMovement|IsFalling (Variables|Character|GetCharacterMovement))
        (Variables|Default|SetState "NewEnumerator2")
        (goto _label)
        (else
          (Variables|Default|SetState "NewEnumerator0")
          (goto _label))))))

(event Input|ActionEvents|InputActionCycleWeaponUp
  (params (Key :type Key%20Structure :default "AnyKey"))
  (:Pressed
    (Variables|Default|SetWeaponIndex (+ (Variables|Default|GetWeaponIndex) 1))
    (if (>= (Variables|Default|GetWeaponIndex) (Variables|Default|GetNumberOfWeapons))
      (Variables|Default|SetWeaponIndex 0)
      (Development|PrintString "Index = 0"))
    (CallFunction|InitWeapon)
    (Development|PrintString (Utilities|String|ToString(Integer) (Variables|Default|GetWeaponIndex)))
    (bind _returnvalue (Utilities|GetDataTableRow "/Game/TutorialProject/Blueprints/WeaponData.WeaponData" (Utilities|Array|Get(acopy) (Variables|Default|GetWeaponArray) (Variables|Default|GetWeaponIndex)))
      (:then
        (Variables|Default|SetWeaponName (.name _returnvalue))
        (Variables|Default|SetWeaponColor (.color _returnvalue))
        (Variables|Default|SetWeaponVelocityX (.velocityx _returnvalue))
        (Variables|Default|SetWeaponVelocityZ (.velocityz _returnvalue))
        (Variables|Default|SetWeaponZRange (.velocityzrange _returnvalue))
        (Variables|Default|SetWeaponProjectileScale (.scale _returnvalue))
        (Variables|Default|SetWeaponFlipbook (.flipbook _returnvalue))
        (Development|PrintString (Variables|Default|GetWeaponName))
        (Development|PrintString (Utilities|String|ToString(Integer) (Variables|Default|GetWeaponColor))))
      (:RowNotFound
        (Development|PrintString "Couldn't Find Row")))))

(event Input|AxisEvents|InputAxisMoveUp
  (params (AxisValue :type Float%20%28single-precision%29))
  ;[0 1 0.2318] Handle Climbing
  (CallFunction|DetectLadder)
  (if (Variables|Default|GetCanClimb)
    (if (Math|Float|InRange(Float) AxisValue -0.1 0.1)
      (if (Utilities|Enum|Equal(Enum) (Variables|Default|GetState) "NewEnumerator8")
        (Components|Movement|StopMovementImmediately (Variables|Character|GetCharacterMovement)))
      (else
        (Variables|Default|SetState "NewEnumerator8")
        (CallFunction|UpdateAnimation)
        (Pawn|Components|CharacterMovement|SetMovementMode (Variables|Character|GetCharacterMovement) "MOVE_Flying" 0)
        (Pawn|Input|AddMovementInput (Math|Vector|MakeVector 0.0 0.0 1.0) (* (Variables|Default|GetClimbSpeed) AxisValue) false)))))

(event Input|AxisEvents|InputAxisMoveRight
  (params (AxisValue :type Float%20%28single-precision%29))
  ;[0 1 0.2318] Handle movement
  (if (Variables|Default|GetCanMove)
    (if (> AxisValue 0.0)
      (Variables|Default|SetisMovingRight true)
      (Variables|Default|SetFacing 1)
      (Pawn|Input|AddMovementInput "1.000000, 0, 0" AxisValue false :!label _label)
      (elif (< AxisValue 0.0)
        (Variables|Default|SetisMovingRight false)
        (Variables|Default|SetFacing -1)
        (goto _label)))))

(event Input|MouseEvents|MouseX
  (params (AxisValue :type Float%20%28single-precision%29)))

(event Input|MouseEvents|MouseY
  (params (AxisValue :type Float%20%28single-precision%29)))

(fn ConstructionScript
  (bind _returnvalue (Rendering|Material|CreateDynamicMaterialInstance (Variables|Default|GetSprite) 0 "/Game/TutorialProject/Materials/PlayerMaterial.PlayerMaterial" :!class /Script/Engine.PrimitiveComponent))
  (Variables|Default|SetSpriteMaterial _returnvalue))

(fn SetWeaponParameters
  (params (Weapon :type BP%20Shot%20Object%20Reference))
  (bind _output_get (Variables|Default|SetWeapon Weapon))
  (Rendering|Material|SetVectorParameterValue (Variables|/Game/TutorialProject/Blueprints/Projectiles/BP_Shot.BP_Shot_C|GetSpriteMaterial _output_get) "Color" (Variables|Default|GetWeaponColor) :!class /Script/Engine.MaterialInstanceDynamic)
  (Rendering|Material|SetScalarParameterValue (Variables|/Game/TutorialProject/Blueprints/Projectiles/BP_Shot.BP_Shot_C|GetSpriteMaterial _output_get) "Scale" (Variables|Default|GetWeaponProjectileScale) :!class /Script/Engine.MaterialInstanceDynamic)
  (return))