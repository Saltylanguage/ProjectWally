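; BP_Ladder is a ladder actor that lets BP_Dude climb while inside its box trigger.
; The construction script stacks paper sprite rungs between LadderBottom and LadderTop, fits the box to that height and places a static mesh at the top.
; Box overlap toggles CanClimb, and leaving also ends climbing and restores the mesh's query and physics collision.
; An AllowDown event jumps into the same cast that enables climbing.
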(event OnComponentBeginOverlap(Box)
  (params (OverlappedComponent :type Primitive%20Component%20Object%20Reference) (OtherActor :type Actor%20Object%20Reference) (OtherComp :type Primitive%20Component%20Object%20Reference) (OtherBodyIndex :type Integer) (bFromSweep :type Boolean) (SweepResult :type Hit%20Result%20Structure%20%28by%20ref%29))
  (bind _asbp_dude (Utilities|Casting|CastToBP_Dude OtherActor))
  (Variables|/Game/TutorialProject/Blueprints/BP_Dude.BP_Dude_C|SetCanClimb _asbp_dude true))

(event OnComponentEndOverlap(Box)
  (params (OverlappedComponent :type Primitive%20Component%20Object%20Reference) (OtherActor :type Actor%20Object%20Reference) (OtherComp :type Primitive%20Component%20Object%20Reference) (OtherBodyIndex :type Integer))
  (bind _asbp_dude (Utilities|Casting|CastToBP_Dude OtherActor))
  (Variables|/Game/TutorialProject/Blueprints/BP_Dude.BP_Dude_C|SetCanClimb _asbp_dude false)
  (Default|ClimbingEnd _asbp_dude)
  (Collision|SetCollisionEnabled (Variables|Default|GetStaticMesh) "QueryAndPhysics"))

(event Custom|AllowDown
  (bind _asbp_dude (Utilities|Casting|CastToBP_Dude (stale OnComponentBeginOverlap(Box) OtherActor)))
  (Variables|/Game/TutorialProject/Blueprints/BP_Dude.BP_Dude_C|SetCanClimb _asbp_dude true))

(event EventBeginPlay)

(event EventActorBeginOverlap
  (params (OtherActor :type Actor%20Object%20Reference)))

(event EventTick
  (params (DeltaSeconds :type Float%20%28single-precision%29)))

(fn ConstructionScript
  (bind _box (Variables|Default|GetBox))
  (bind _laddertop (Variables|Default|GetLadderTop))
  (bind _ladderbottom (Variables|Default|GetLadderBottom))
  (bind _rungoffset (Variables|Default|GetRungOffset))
  (bind _staticmesh (Variables|Default|GetStaticMesh))
  (bind _returnvalue (- _laddertop _ladderbottom))
  (bind _returnvalue_2 (/ (.z _returnvalue) 2.0))
  (Utilities|FlowControl|Sequence
    (:then_0
      (for _index (range 0 (Math|Float|Truncate (/ (.z _returnvalue) _rungoffset)))
        (bind _returnvalue_3 (AddComponent|AddPaperSpriteComponent false (Math|Transform|MakeTransform (Math|Vector|MakeVector 0.0 0.0 (* _index _rungoffset)) "0, 0, 0" "1,1,1")))
        (Rendering|Components|Sprite|SetSprite _returnvalue_3 (Variables|Default|GetLadderSprite))
        (Collision|SetCollisionEnabled _returnvalue_3 "NoCollision"))
      (Transformation|SetRelativeScale3D _box (Math|Vector|MakeVector (Variables|Default|GetCollisionWidth) 1.0 _returnvalue_2))
      (Transformation|SetRelativeLocation _box (Math|Vector|MakeVector 0.0 0.0 _returnvalue_2) false false))
    (:then_1
      (Transformation|SetRelativeScale3D _staticmesh (Math|Vector|MakeVector (Variables|Default|GetCollisionWidth) 2e+01 1.0))
      (Transformation|SetRelativeLocation _staticmesh (Variables|Default|GetLadderTop) false false))))