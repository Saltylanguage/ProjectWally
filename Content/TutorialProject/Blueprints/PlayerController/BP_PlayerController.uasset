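; Player controller that fires BP_Shot projectiles toward the mouse cursor while the left mouse button is held.
; It caches the controlled BP_Player on BeginPlay, and the mouse button opens and closes a gate on Tick, where a short Delay throttles spawning.
; Each shot spawns at the player's Arrow and heads at initial speed toward the deprojected cursor position, with the target's Y zeroed for XZ-plane aiming.
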(event EventBeginPlay
  (bind _asbp_player (Utilities|Casting|CastToBP_Player (Pawn|GetControlledPawn)))
  (Variables|Default|SetPlayerPawn _asbp_player))

(event EventTick
  (params (DeltaSeconds :type Float%20%28single-precision%29))
  (bind _worldlocation (Game|Player|ConvertMouseLocationToWorldSpace))
  (bind _playerpawn (Variables|Default|GetPlayerPawn))
  (bind _arrow (Variables|/Game/TutorialProject/Blueprints/Player/BP_Player.BP_Player_C|GetArrow _playerpawn))
  (bind _returnvalue (Transformation|GetWorldLocation _arrow))
  (Utilities|FlowControl|Gate true
    (:Exit
      (Utilities|FlowControl|Delay 0.1)
      (bind _returnvalue_2 (Game|SpawnActorfromClass "/Game/TutorialProject/Blueprints/Projectiles/BP_Shot.BP_Shot_C" (Math|Transform|MakeTransform _returnvalue "0, 0, 0" "1.000000,1,1") "Undefined" 0 0))
      (Variables|/Script/Engine.MovementComponent|SetVelocity (Variables|/Game/TutorialProject/Blueprints/Projectiles/BP_Shot.BP_Shot_C|GetProjectileMovement _returnvalue_2) (* (Math|Vector|Normalize (- (Math|Vector|MakeVector (.x _worldlocation) 0.0 (.z _worldlocation)) _returnvalue)) (Variables|/Script/Engine.ProjectileMovementComponent|GetInitialSpeed (Variables|/Game/TutorialProject/Blueprints/Projectiles/BP_Shot.BP_Shot_C|GetProjectileMovement _returnvalue_2)))))))

(event Input|MouseEvents|LeftMouseButton
  (params (Key :type Key%20Structure :default "AnyKey"))
  (bind _worldlocation (Game|Player|ConvertMouseLocationToWorldSpace))
  (bind _playerpawn (Variables|Default|GetPlayerPawn))
  (bind _arrow (Variables|/Game/TutorialProject/Blueprints/Player/BP_Player.BP_Player_C|GetArrow _playerpawn))
  (bind _returnvalue (Transformation|GetWorldLocation _arrow))
  (:Pressed
    (Utilities|FlowControl|Gate true) ; enters at Open
  )
  (:Released
    (Utilities|FlowControl|Gate true) ; enters at Close
  ))

(fn ConstructionScript)